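; BP_P38 is an aircraft actor, named for the P-38, that flies straight ahead with spinning propellers.
; Each Tick rolls the left and right propeller components at a fixed rate and offsets the actor along its local X axis at constant speed.
; Both motions scale with world delta seconds to stay frame-rate independent, and the construction script is empty.
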(event EventTick
  (params (DeltaSeconds :type Float%20%28single-precision%29))
  (Transformation|AddLocalRotation (Variables|Default|GetL_Propeller) (Math|Rotator|MakeRotator (* 3.6e+03 (Utilities|Time|GetWorldDeltaSeconds)) 0.0 0.0) false false)
  (Transformation|AddLocalRotation (Variables|Default|GetR_Propeller) (Math|Rotator|MakeRotator (* 3.6e+03 (Utilities|Time|GetWorldDeltaSeconds)) 0.0 0.0) false false)
  (Transformation|AddActorLocalOffset (Math|Vector|MakeVector (* (Utilities|Time|GetWorldDeltaSeconds) 1e+02) 0.0 0.0) false false))

(fn ConstructionScript)