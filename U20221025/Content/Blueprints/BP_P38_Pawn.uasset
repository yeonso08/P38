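; BP_P38_Pawn is a player-controlled P-38 plane pawn that constantly flies forward with spinning propellers.
; Roll and Pitch axes rotate it locally, frame-rate scaled, while Boost raises the FloatingPawnMovement max speed until released.
; Fire spawns a BP_ROC missile at the Arrow component.
; Any actor overlap spawns an explosion effect and sound, then destroys the plane.
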(event Collision|EventActorBeginOverlap
  (params (OtherActor :type Actor%20Object%20Reference))
  ;[1 1 1] 부딪히면 파괴
  (Effects|SpawnEmitteratLocation "/Game/StarterContent/Particles/P_Explosion.P_Explosion" (Transformation|GetActorLocation))
  (Audio|SpawnSoundatLocation "/Game/StarterContent/Audio/Explosion_Cue.Explosion_Cue" (Transformation|GetActorLocation) "0, 0, 0" 1.0 1.0 0.0 0 0)
  (Actor|DestroyActor))

(event EventTick
  (params (DeltaSeconds :type Float%20%28single-precision%29))
  ;[1 1 1] 프로펠라 회전
  (Transformation|AddLocalRotation (Variables|Default|GetL_Propeller) (Math|Rotator|MakeRotator (* 3.6e+03 (Utilities|Time|GetWorldDeltaSeconds)) 0.0 0.0) false false)
  (Transformation|AddLocalRotation (Variables|Default|GetR_Propeller) (Math|Rotator|MakeRotator (* 3.6e+03 (Utilities|Time|GetWorldDeltaSeconds)) 0.0 0.0) false false)
  ;[1 1 1] 이동
  (Pawn|Input|AddMovementInput (Transformation|GetActorForwardVector) 1.0 false))

(event Input|ActionEvents|InputActionBoost
  (params (Key :type Key%20Structure :default "None"))
  ;[1 1 1] Boost 입력키
  (:Pressed
    (bind _output_get (Variables|Default|SetBoostSpeed 8e+02))
    (Variables|/Script/Engine.FloatingPawnMovement|SetMaxSpeed (Variables|Default|GetFloatingPawnMovement) _output_get))
  (:Released
    (bind _output_get_2 (Variables|Default|SetBoostSpeed 1e+02))
    (Variables|/Script/Engine.FloatingPawnMovement|SetMaxSpeed (Variables|Default|GetFloatingPawnMovement) _output_get_2)))

(event Input|ActionEvents|InputActionFire
  (params (Key :type Key%20Structure :default "None"))
  ;[1 1 1] 미사일 나가기
  (:Pressed
    (Game|SpawnActorfromClass "/Game/Blueprints/BP_ROC.BP_ROC_C" (Transformation|GetWorldTransform (Variables|Default|GetArrow)) "Undefined" 0 0)))

(event Input|AxisEvents|InputAxisPitch
  (params (AxisValue :type Float%20%28single-precision%29))
  ;[1 1 1] Pitch 회전
  (Transformation|AddActorLocalRotation (Math|Rotator|MakeRotator 0.0 (* (Math|Float|Clamp(Float) AxisValue -1.0) (Utilities|Time|GetWorldDeltaSeconds) (Variables|Default|GetRotaionSpeed)) 0.0) false false))

(event Input|AxisEvents|InputAxisRoll
  (params (AxisValue :type Float%20%28single-precision%29))
  ;[1 1 1] Roll ㅚ전
  (Transformation|AddActorLocalRotation (Math|Rotator|MakeRotator (* (Math|Float|Clamp(Float) AxisValue -1.0) (Utilities|Time|GetWorldDeltaSeconds) (Variables|Default|GetRotaionSpeed)) 0.0 0.0) false false))

(fn ConstructionScript)