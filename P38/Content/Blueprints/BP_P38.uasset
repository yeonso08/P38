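; BP_P38 is a player-controllable P-38 airplane with spinning left and right propellers.
; Each Tick rolls both propellers, Right through the RotatePropeller function and Left inline, then moves the actor along world X without sweep.
; Roll and Pitch axis inputs apply frame-time-scaled local rotation to the actor.
; Movement ignores the actor's orientation, so rotating the plane does not change its travel direction.
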(event EventTick
  (params (DeltaSeconds :type Float%20%28single-precision%29))
  ;[1 1 1] Right 회전
  (CallFunction|RotatePropeller (Variables|Default|GetRight))
  ;[1 1 1] Left 회전
  (Transformation|AddLocalRotation (Variables|Default|GetLeft) (Math|Rotator|MakeRotator (* (Utilities|Time|GetWorldDeltaSeconds) (Variables|Default|GetPropellaRotationSpeed)) 0.0 0.0) false false)
  ;[1 1 1] 비행기이동
  (Transformation|AddActorWorldOffset (Math|Vector|MakeVector (* (Utilities|Time|GetWorldDeltaSeconds) (Variables|Default|GetMoveSpeed)) 0.0 0.0)))

(event Input|AxisEvents|InputAxisRoll
  (params (AxisValue :type Float%20%28single-precision%29))
  (Transformation|AddActorLocalRotation (Math|Rotator|MakeRotator (* AxisValue (Variables|Default|GetRotationSpped) (Utilities|Time|GetWorldDeltaSeconds)) 0.0 0.0) false false))

(event Input|AxisEvents|InputAxisPitch
  (params (AxisValue :type Float%20%28single-precision%29))
  (Transformation|AddActorLocalRotation (Math|Rotator|MakeRotator 0.0 (* AxisValue (Variables|Default|GetRotationSpped) (Utilities|Time|GetWorldDeltaSeconds)) 0.0) false false))

(fn ConstructionScript)

(fn RotatePropeller
  (params (self2 :type Scene%20Component%20Object%20Reference))
  (Transformation|AddLocalRotation self2 (Math|Rotator|MakeRotator (* (Utilities|Time|GetWorldDeltaSeconds) (Variables|Default|GetPropellaRotationSpeed)) 0.0 0.0) false false))